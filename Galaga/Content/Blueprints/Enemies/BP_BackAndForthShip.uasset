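; BP_BackAndForthShip is an enemy ship that moves back and forth along the Z axis, making net progress toward negative Z.
; Each Tick, while MoveEnabled is set, a swept SetActorLocation steps it toward TargetLocation at Speed.
; Reaching the target's Z flips GoingForth and sets a new target relative to the current position, with longer downward legs than upward ones.
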(event `self.ReceiveBeginPlay`
  (`parent.ReceiveBeginPlay`)
  (set `self.TargetLocation` (`self.K2_GetActorLocation`)))

(event `self.ReceiveTick`
  (params (DeltaSeconds :type "Float (single-precision)"))
  (`self.BackAndForthMove` DeltaSeconds))

(fn `BackAndForthMove`
  (params (DeltaSeconds :type "Float (double-precision)"))
  (bind (_returnvalue_x _returnvalue_y _returnvalue_z) (`KismetMathLibrary.BreakVector` (`self.K2_GetActorLocation`)))
  (bind (_returnvalue_x_2 _returnvalue_y_2 _returnvalue_z_2) (`KismetMathLibrary.BreakVector` (`self.K2_GetActorLocation`)))
  (bind (_targetlocation_x _targetlocation_y _targetlocation_z) (`KismetMathLibrary.BreakVector` (`self.TargetLocation`)))
  (bind (_targetlocation_x_2 _targetlocation_y_2 _targetlocation_z_2) (`KismetMathLibrary.BreakVector` (`self.TargetLocation`)))
  (if (== (`self.MoveEnabled`) true)
    (`self.K2_SetActorLocation` (+ (* (* (`KismetMathLibrary.Normal` (- (`self.TargetLocation`) (`self.K2_GetActorLocation`))) DeltaSeconds) (`self.Speed`)) (`self.K2_GetActorLocation`)) true)
    (if (`self.GoingForth`)
      (if (<= _returnvalue_z_2 _targetlocation_z_2)
        (set `self.GoingForth` (not (`self.GoingForth`)) :!label _label)
        (if (`self.GoingForth`)
          (set `self.TargetLocation` (+ (0.0 0.0 -45.0) (`self.K2_GetActorLocation`)))
          (else
            (set `self.TargetLocation` (+ (0.0 0.0 15.0) (`self.K2_GetActorLocation`))))))
      (elif (>= _returnvalue_z _targetlocation_z)
        (goto _label)))))

(fn `UserConstructionScript`
  (`parent.UserConstructionScript`))