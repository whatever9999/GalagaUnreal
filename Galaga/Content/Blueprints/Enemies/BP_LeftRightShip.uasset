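; BP_LeftRightShip is an enemy ship that descends in a zigzag, alternating diagonal legs along X while dropping in Z.
; Each Tick, LeftRightMove calls MoveTowardTarget when MoveEnabled is set, then tests whether the current target has been reached.
; On arrival it flips GoingLeft and offsets a new target by AmountToMove from the current location.
; The target starts at the spawn location, seeded on BeginPlay.
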(event `self.ReceiveBeginPlay`
  ;[1 1 1] Set initial target location
  (`parent.ReceiveBeginPlay`)
  (set `self.TargetLocation` (`self.K2_GetActorLocation`)))

(event `self.ReceiveTick`
  (params (DeltaSeconds :type "Float (single-precision)"))
  ;[1 1 1] Move
  (`self.LeftRightMove` DeltaSeconds))

(fn `LeftRightMove`
  (params (DeltaSeconds :type "Float (double-precision)"))
  (locals (AmountToMove :type "Float (double-precision)" :default 40.0))
  (bind (_returnvalue_x _returnvalue_y _returnvalue_z) (`KismetMathLibrary.BreakVector` (`self.K2_GetActorLocation`)))
  (bind (_returnvalue_x_2 _returnvalue_y_2 _returnvalue_z_2) (`KismetMathLibrary.BreakVector` (`self.K2_GetActorLocation`)))
  (bind _amounttomove (`local.AmountToMove`))
  (bind (_targetlocation_x _targetlocation_y _targetlocation_z) (`KismetMathLibrary.BreakVector` (`self.TargetLocation`)))
  (bind (_targetlocation_x_2 _targetlocation_y_2 _targetlocation_z_2) (`KismetMathLibrary.BreakVector` (`self.TargetLocation`)))
  (bind _returnvalue (* -1 (`local.AmountToMove`)))
  ;[1 1 1] If ship can move, move it
  (if (== (`self.MoveEnabled`) true)
    (`self.MoveTowardTarget` (`self.TargetLocation`) DeltaSeconds)
    ;[1 1 1] Check if ship has reached target - if it has then set new target
    (if (`self.GoingLeft`)
      (if (and (>= _returnvalue_x _targetlocation_x) (<= _returnvalue_z _targetlocation_z))
        (set `self.GoingLeft` (not (`self.GoingLeft`)) :!label _label)
        (if (`self.GoingLeft`)
          (set `self.TargetLocation` (+ (`KismetMathLibrary.MakeVector` _amounttomove 0.0 (* -1 _amounttomove)) (`self.K2_GetActorLocation`)))
          (else
            (set `self.TargetLocation` (+ (`KismetMathLibrary.MakeVector` _returnvalue 0.0 _returnvalue) (`self.K2_GetActorLocation`))))))
      (elif (and (<= _returnvalue_x_2 _targetlocation_x_2) (<= _returnvalue_z_2 _targetlocation_z_2))
        (goto _label)))))

(fn `UserConstructionScript`
  (`parent.UserConstructionScript`))