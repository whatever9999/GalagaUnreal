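; Base enemy ship for a scrolling shooter, sliding in on a spawn timeline and then moving straight down the screen.
; Die plays an explosion flipbook and sound, randomly drops a life or rocket pickup, destroys the actor and reports points to BP_GameMode.
; Hit explodes the ship without points or drops, with sound only against the player.
; MoveTowardTarget offers homing movement but is unused here.
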(event `self.ReceiveBeginPlay`
  (bind _spawnlocation (`self.SpawnLocation`))
  ;[1 1 1] Set Up References and Variables
  (bind _asbp_game_mode (cast `/Game/Blueprints/BP_GameMode` (`GameplayStatics.GetGameMode`)))
  (set `self.BP_GameMode` _asbp_game_mode)
  (set `self.CurrentSpeed` (`self.Speed`))
  (set `self.SpawnLocation` (`self.K2_GetActorLocation`))
  ;[1 1 1] Spawn
  (bind (_direction _entryspeed) (`Timeline|SpawnAnimation`)
    (:`Update`
      (`self.K2_SetActorLocation` (`KismetMathLibrary.VLerp` _spawnlocation (- _spawnlocation (`KismetMathLibrary.MakeVector` 0.0 0.0 (`self.SpawnZ`))) _entryspeed))
      (`SceneComponent.SetVisibility` (`self.Explosion`) false false))
    (:`Finished`
      (set `self.MoveEnabled` true))))

(event `self.ReceiveTick`
  (params (DeltaSeconds :type "Float (single-precision)"))
  ;[1 1 1] Movement
  (`self.StraightMovement` DeltaSeconds))

(event `Die`
  (bind _explosion (`self.Explosion`))
  ;[1 1 1] Die
  (`PrimitiveComponent.SetCollisionResponseToAllChannels` (`self.Enemy`) "ECR_Ignore")
  (`SceneComponent.SetVisibility` (`self.Explosion`) true false)
  (`PaperFlipbookComponent.PlayFromStart` _explosion)
  (`GameplayStatics.PlaySound2D` "/Game/Assets/SFX/WAV/Explosion2.Explosion2" 1.0 1.0 0.0 null null)
  (`self.Drop`)
  (`KismetSystemLibrary.Delay` (`PaperFlipbookComponent.GetFlipbookLength` _explosion))
  (`self.K2_DestroyActor`)
  (`/Game/Blueprints/BP_GameMode.SetScore` (`self.BP_GameMode`) (`self.PointsForDeath`)))

(event `self.ReceiveHit`
  (params (MyComp :type "PrimitiveComponent Object Reference") (Other :type "Actor Object Reference") (OtherComp :type "PrimitiveComponent Object Reference") (bSelfMoved :type Boolean) (HitLocation :type "Vector Structure") (HitNormal :type "Vector Structure") (NormalImpulse :type "Vector Structure") (Hit :type "HitResult Structure (by ref)"))
  (bind _explosion (`self.Explosion`))
  ;[1 1 1] Ship collides with a non-projectile (E.g. player or bounding walls)
  (cast `/Game/Blueprints/BP_Player` Other
    (:`then`
      (`GameplayStatics.PlaySound2D` "/Game/Assets/SFX/WAV/Explosion2.Explosion2" 1.0 1.0 0.0 null null))
    (:`CastFailed`
      _))
  (`PrimitiveComponent.SetCollisionResponseToAllChannels` (`self.Enemy`) "ECR_Ignore")
  (`SceneComponent.SetVisibility` (`self.Explosion`) true false)
  (`PaperFlipbookComponent.PlayFromStart` _explosion)
  (`KismetSystemLibrary.Delay` (`PaperFlipbookComponent.GetFlipbookLength` _explosion))
  (`self.K2_DestroyActor`))

(fn `Drop`
  (locals (ChanceToDropLife :type "Float (double-precision)" :default 5.0) (ChanceToDropRocket :type "Float (double-precision)" :default 25.0))
  ;[1 1 1] Randomly check to see if a life or rocket is dropped
  (set `self.DropLife` (`KismetMathLibrary.RandomBool`))
  (if (`self.DropLife`)
    (if (< (`KismetMathLibrary.RandomFloatInRange` 0.0 100.0) (`local.ChanceToDropLife`))
      (`|SpawnActorFromClass` "/Game/Blueprints/Droppables/BP_Life.BP_Life_C" (`self.GetTransform`) "Undefined" "OverrideRootScale" null null))
    (elif (< (`KismetMathLibrary.RandomFloatInRange` 0.0 100.0) (`local.ChanceToDropRocket`))
      (`|SpawnActorFromClass` "/Game/Blueprints/Droppables/BP_EnemyRocket.BP_EnemyRocket_C" (`self.GetTransform`) "Undefined" "OverrideRootScale" null null))))

(fn `MoveTowardTarget`
  (params (Target :type "Vector Structure") (DeltaSeconds :type "Float (double-precision)"))
  ;[1 1 1] Make movement (for a frame) towards target
  (`self.K2_SetActorLocation` (+ (* (* (`KismetMathLibrary.Normal` (- Target (`self.K2_GetActorLocation`))) DeltaSeconds) (`self.Speed`)) (`self.K2_GetActorLocation`)) true))

(fn `StraightMovement`
  (params (DeltaSeconds :type "Float (double-precision)"))
  ;[1 1 1] Move in straight line down screen
  (if (== (`self.MoveEnabled`) true)
    (`self.K2_SetActorLocation` (+ (`self.K2_GetActorLocation`) (* (`KismetMathLibrary.MakeVector` 0.0 0.0 (* (`self.CurrentSpeed`) -1.0)) DeltaSeconds)) true)))

(fn `UserConstructionScript`)