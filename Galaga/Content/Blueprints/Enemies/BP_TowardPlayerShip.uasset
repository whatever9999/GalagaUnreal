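; Enemy ship Blueprint that homes in on the player's position.
; Each Tick calls TowardPlayerMove, which, while MoveEnabled is set, steps along the normalized direction to player pawn 0, scaled by Speed and delta time, using a swept move.
; The ship does not rotate, and it falls back to StraightMovement when that pawn does not match BP_Player.
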(event `self.ReceiveTick`
  (params (DeltaSeconds :type "Float (single-precision)"))
  (`self.TowardPlayerMove` DeltaSeconds))

(fn `TowardPlayerMove`
  (params (DeltaSeconds :type "Float (double-precision)"))
  (if (== (`self.MoveEnabled`) true)
    (if (== (`GameplayStatics.GetPlayerPawn` 0) "/Game/Blueprints/BP_Player.BP_Player")
      (`self.K2_SetActorLocation` (+ (* (* (`KismetMathLibrary.Normal` (- (`self.K2_GetActorLocation` (`GameplayStatics.GetPlayerPawn` 0)) (`self.K2_GetActorLocation`))) DeltaSeconds) (`self.Speed`)) (`self.K2_GetActorLocation`)) true)
      (else
        (`self.StraightMovement` DeltaSeconds)))))

(fn `UserConstructionScript`
  (`parent.UserConstructionScript`))