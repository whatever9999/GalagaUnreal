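; BP_GameMode is the game mode that tracks the player's score and manages the HUD and game-over screen.
; On BeginPlay it switches input to game-only, initializes the score and adds the BPW_HUD widget to the viewport.
; SetScore adds the passed amount to the running total rather than replacing it.
; GameOver shows BPW_GameOver for restart or exit, enables the cursor and switches input to UI-only focused on that widget.
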(event `self.ReceiveBeginPlay`
  ;[1 1 1] Make cursor disappear on startup
  (`WidgetBlueprintLibrary.SetInputMode_GameOnly` (`GameplayStatics.GetPlayerController` 0))
  ;[1 1 1] Make HUD visible
  (`self.SetScore` 0)
  (bind _returnvalue (`|CreateWidget` "/Game/Blueprints/Widgets/BPW_HUD.BPW_HUD_C"))
  (bind _output_get (set `self.BPW_HUD` _returnvalue))
  (`UserWidget.AddToViewport` _output_get 0))

(fn `GameOver`
  (bind _returnvalue (`GameplayStatics.GetPlayerController` 0))
  ;[1 1 1] Create BPW_GameOver Widget to allow player to exit/restart
  (bind _returnvalue_2 (`|CreateWidget` "/Game/Blueprints/Widgets/BPW_GameOver.BPW_GameOver_C"))
  (`UserWidget.AddToViewport` _returnvalue_2 0)
  (set `PlayerController.bShowMouseCursor` true _returnvalue)
  (`WidgetBlueprintLibrary.SetInputMode_UIOnlyEx` _returnvalue _returnvalue_2))

(fn `SetScore`
  (params (addScore :type Integer))
  ;[1 1 1] Update the score
  (set `self.Score` (+ addScore (`self.Score`))))

(fn `UserConstructionScript`)