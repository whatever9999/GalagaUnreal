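; Base player projectile that kills enemies it overlaps and applies a score penalty when it overlaps anything else.
; An overlap with a BP_EnemyBase calls Die on it, while any other overlap passes TakeawayPoints to SetScore on the BP_GameMode cached at BeginPlay.
; The projectile destroys itself in both cases.
; The construction script drives the movement component's initial and max speed from the Speed variable.
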(event `self.ReceiveBeginPlay`
  ;[1 1 1] Get game mode
  (bind _asbp_game_mode (cast `/Game/Blueprints/BP_GameMode` (`GameplayStatics.GetGameMode`)))
  (set `self.GameMode` _asbp_game_mode))

(event `self.Projectile.OnComponentBeginOverlap`
  (params (OverlappedComponent :type "PrimitiveComponent Object Reference") (OtherActor :type "Actor Object Reference") (OtherComp :type "PrimitiveComponent Object Reference") (OtherBodyIndex :type Integer) (bFromSweep :type Boolean) (SweepResult :type "HitResult Structure (by ref)"))
  ;[1 1 1] If projectile hits enemy then kill it and destroy self, otherwise lose points and destroy self (if collides with bounding box)
  (bind _asbp_enemy_base (cast `/Game/Blueprints/Enemies/BP_EnemyBase` OtherActor)
    (:`then`
      (`/Game/Blueprints/Enemies/BP_EnemyBase.Die` _asbp_enemy_base)
      (`self.K2_DestroyActor`))
    (:`CastFailed`
      (`/Game/Blueprints/BP_GameMode.SetScore` (`self.GameMode`) (`self.TakeawayPoints`))
      (`self.K2_DestroyActor`))))

(fn `UserConstructionScript`
  (bind _projectilemovement (`self.ProjectileMovement`))
  ;[1 1 1] Move
  (bind _output_get (set `ProjectileMovementComponent.MaxSpeed` (`self.Speed`) _projectilemovement))
  (set `ProjectileMovementComponent.InitialSpeed` _output_get _projectilemovement))