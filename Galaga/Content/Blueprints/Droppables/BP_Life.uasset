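; BP_Life is a droppable pickup that grants the player an extra life.
; When an actor overlaps it, it casts that actor to BP_Player, stores the reference, increments the player's Lives and destroys itself.
; Actors that are not BP_Player are ignored, and BeginPlay, Tick and the construction script add no logic.
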(event `self.ReceiveActorBeginOverlap`
  (params (OtherActor :type "Actor Object Reference"))
  ;[1 1 1] Add a life to player and destroy self
  (bind _asbp_player (cast `/Game/Blueprints/BP_Player` OtherActor))
  (bind _output_get (set `self.Player` _asbp_player))
  (bind _result (`/Engine/EditorBlueprintResources/StandardMacros.IncrementInt` (`/Game/Blueprints/BP_Player.Lives` _output_get))
    (:`  `
      (set `/Game/Blueprints/BP_Player.Lives` _result (`self.Player`))
      (`self.K2_DestroyActor`))))

(fn `UserConstructionScript`
  (`parent.UserConstructionScript`))