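; Player actor for a shooter: it slides along the X axis, fires weapons and loses lives when hit.
; Axis input eases a speed value that Tick applies as a swept move.
; Looping timers repeat single rocket, triple rocket and laser fire while held; single rocket alone skips the immediate shot.
; Enemy or enemy-rocket hits cost a life, triggering blinking invulnerability via collision-channel toggling, or GameMode game over once lives drop below zero.
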(event `self.ReceiveBeginPlay`
  ;[1 1 1] Spawn player
  (bind _asbp_game_mode (cast `/Game/Blueprints/BP_GameMode` (`GameplayStatics.GetGameMode`)))
  (set `self.BP_GameMode` _asbp_game_mode))

(event `InputAxis|Move`
  (params (AxisValue :type "Float (single-precision)"))
  ;[1 1 1] Player movement input
  (bind _newspeed (`self.Movement` (`self.CurrentSpeed`) AxisValue))
  (set `self.CurrentSpeed` _newspeed))

(event `self.ReceiveTick`
  (params (DeltaSeconds :type "Float (single-precision)"))
  ;[1 1 1] Movement
  (set `self.DeltaSeconds` DeltaSeconds)
  (`self.K2_SetActorLocation` (+ (`self.K2_GetActorLocation`) (`KismetMathLibrary.MakeVector` (`self.CurrentSpeed`))) true))

(event `InputAction|Single Rocket`
  (params (Key :type "Key Structure"))
  ;[1 1 1] Single Rocket
  (:`Pressed`
    (`KismetSystemLibrary.K2_SetTimer` null "SingleRocketShoot" (`self.SingleRocketTimeBetweenShots`) true))
  (:`Released`
    (`KismetSystemLibrary.K2_ClearTimer` null "SingleRocketShoot")))

(event `InputAction|Triple Rocket`
  (params (Key :type "Key Structure"))
  ;[1 1 1] Triple rocket input
  (:`Pressed`
    (`KismetSystemLibrary.K2_SetTimer` null "RocketShoot" (`self.TimeBetweenShots`) true)
    (`self.TripleRocket` (`SceneComponent.K2_GetComponentToWorld` (`self.RocketSpawn`)) (`SceneComponent.K2_GetComponentToWorld` (`self.Rocket2Spawn`)) (`SceneComponent.K2_GetComponentToWorld` (`self.Rocket3Spawn`)) :!label _label))
  (:`Released`
    (`KismetSystemLibrary.K2_ClearTimer` null "RocketShoot")))

(event `SingleRocketShoot`
  ;[1 1 1] Single Rocket
  (`self.SingleRocket` (`SceneComponent.K2_GetComponentToWorld` (`self.RocketSpawn`))))

(event `RocketShoot`
  ;[1 1 1] Triple rocket input
  (goto _label))

(event `InputAction|Laser`
  (params (Key :type "Key Structure"))
  ;[1 1 1] Laser input
  (:`Pressed`
    (`KismetSystemLibrary.K2_SetTimer` null "LaserShoot" (`self.TimeBetweenShots`) true)
    (`self.Laser` (`SceneComponent.K2_GetComponentToWorld` (`self.LaserSpawn`)) :!label _label_2))
  (:`Released`
    (`KismetSystemLibrary.K2_ClearTimer` null "LaserShoot")))

(event `LaserShoot`
  ;[1 1 1] Laser input
  (goto _label_2))

(event `self.ReceiveHit`
  (params (MyComp :type "PrimitiveComponent Object Reference") (Other :type "Actor Object Reference") (OtherComp :type "PrimitiveComponent Object Reference") (bSelfMoved :type Boolean) (HitLocation :type "Vector Structure") (HitNormal :type "Vector Structure") (NormalImpulse :type "Vector Structure") (Hit :type "HitResult Structure (by ref)"))
  ;[1 1 1] Player reaction to hit (Check to see if enemy and act accordingly, checking to see if dead)
  (cast `/Game/Blueprints/Enemies/BP_EnemyBase` Other
    (:`then`
      _)
    (:`CastFailed`
      (cast `/Game/Blueprints/Droppables/BP_EnemyRocket` Other)))
  (`PrimitiveComponent.SetCollisionResponseToChannel` (`self.PlayerSprite`) "ECC_GameTraceChannel1" "ECR_Ignore")
  (bind _nolivesleft (`self.CheckLives`))
  (if _nolivesleft
    (`/Game/Blueprints/BP_GameMode.GameOver` (`self.BP_GameMode`))
    (`self.K2_DestroyActor`)
    (else
      (if (== (`self.LoopIndex`) 3) :!label _label_3
        (set `self.LoopIndex` 0)
        (`PrimitiveComponent.SetCollisionResponseToChannel` (`self.PlayerSprite`) "ECC_GameTraceChannel1" "ECR_Block")
        (else
          ;[1 1 1] Blink effect
          (`SceneComponent.SetVisibility` (`self.PlayerSprite`) false false)
          (`KismetSystemLibrary.Delay` (`self.TimeBetweenBlinks`))
          (`SceneComponent.SetVisibility` (`self.PlayerSprite`) true false)
          (`KismetSystemLibrary.Delay` (`self.TimeBetweenBlinks`))
          (`/Engine/EditorBlueprintResources/StandardMacros.IncrementInt` (`self.LoopIndex`)
            (:`  `
              (goto _label_3))))))))

(fn `CheckLives`
  (returns (NoLivesLeft :type Boolean))
  (bind _lives (`self.Lives`))
  ;[1 1 1] Check if player has run out of lives
  (`/Engine/EditorBlueprintResources/StandardMacros.DecrementInt` _lives
    (:`  `
      (return (< _lives 0)))))

(fn `Laser`
  (params (Spawn :type "Transform Structure"))
  ;[1 1 1] Spawn laser
  (`|SpawnActorFromClass` "/Game/Blueprints/Projectiles/BP_Laser.BP_Laser_C" Spawn "AlwaysSpawn" "OverrideRootScale" null self)
  (`GameplayStatics.PlaySound2D` "/Game/Assets/SFX/WAV/Rocket.Rocket" 1.0 1.0 0.0 null null))

(fn `Movement`
  (params (CurrentSpeed :type "Float (double-precision)") (UserInput :type "Float (double-precision)"))
  (returns (NewSpeed :type "Float (double-precision)"))
  ;[1 1 1] Move Player according to input
  (return (`KismetMathLibrary.FInterpTo` CurrentSpeed (* (* UserInput (`self.MaxSpeed`)) (`self.DeltaSeconds`)) (`self.DeltaSeconds`) 3.0)))

(fn `SingleRocket`
  (params (Spawn :type "Transform Structure"))
  ;[1 1 1] Spawn a single rocket
  (`|SpawnActorFromClass` "/Game/Blueprints/Projectiles/BP_Rocket.BP_Rocket_C" Spawn "AlwaysSpawn" "OverrideRootScale" null self)
  (`GameplayStatics.PlaySound2D` "/Game/Assets/SFX/WAV/Rocket.Rocket" 1.0 1.0 0.0 null null))

(fn `TripleRocket`
  (params (SpawnRocket :type "Transform Structure") (SpawnRocket2 :type "Transform Structure") (SpawnRocket3 :type "Transform Structure"))
  ;[1 1 1] Spawn triple rocket
  (`|SpawnActorFromClass` "/Game/Blueprints/Projectiles/BP_Rocket.BP_Rocket_C" SpawnRocket "AlwaysSpawn" "OverrideRootScale" null self)
  (`|SpawnActorFromClass` "/Game/Blueprints/Projectiles/BP_Rocket.BP_Rocket_C" SpawnRocket2 "AlwaysSpawn" "OverrideRootScale" null self)
  (`|SpawnActorFromClass` "/Game/Blueprints/Projectiles/BP_Rocket.BP_Rocket_C" SpawnRocket3 "AlwaysSpawn" "OverrideRootScale" null self)
  (`GameplayStatics.PlaySound2D` "/Game/Assets/SFX/WAV/Rocket.Rocket" 1.0 1.0 0.0 null null))

(fn `UserConstructionScript`
  (set `self.Lives` (`self.MaxLives`)))